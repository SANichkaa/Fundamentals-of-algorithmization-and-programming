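; Enemy spawner that creates desert enemies (Snake, Scorpio, Vulture, Hyena, Mummy) just above its own location on a timer.
; Each tick re-arms the timer slightly shorter until the interval bottoms out around three seconds.
; SpawnCode takes the last spawned type and selects the next, with Mummy as the fallback.
; Every tick also raises all five enemy HP values stored on the HealthAndGold player character, scaling difficulty over time.
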(event Custom|Spawn%20Tick
  (if (> (Variables|Default|GetMyTime) 3.0)
    (CallFunction|TimerReset))
  (bind _returnvalue (Class|Spawn|SpawnCode (Variables|Default|GetLast_Enemy)))
  (bind _ashealth_and_gold (Utilities|Casting|CastToHealthAndGold (Game|GetPlayerCharacter 0)))
  (Variables|/Game/BluePrints/Interface/HealthAndGold.HealthAndGold_C|SetHpHyena _ashealth_and_gold (+ (Variables|/Game/BluePrints/Interface/HealthAndGold.HealthAndGold_C|GetHpHyena _ashealth_and_gold) 1))
  (Variables|/Game/BluePrints/Interface/HealthAndGold.HealthAndGold_C|SetHpMummy _ashealth_and_gold (+ (Variables|/Game/BluePrints/Interface/HealthAndGold.HealthAndGold_C|GetHpMummy _ashealth_and_gold) 1))
  (Variables|/Game/BluePrints/Interface/HealthAndGold.HealthAndGold_C|SetHpScorpio _ashealth_and_gold (+ (Variables|/Game/BluePrints/Interface/HealthAndGold.HealthAndGold_C|GetHpScorpio _ashealth_and_gold) 1))
  (Variables|/Game/BluePrints/Interface/HealthAndGold.HealthAndGold_C|SetHpSnake _ashealth_and_gold (+ (Variables|/Game/BluePrints/Interface/HealthAndGold.HealthAndGold_C|GetHpSnake _ashealth_and_gold) 1))
  (Variables|/Game/BluePrints/Interface/HealthAndGold.HealthAndGold_C|SetHpVultur _ashealth_and_gold (+ (Variables|/Game/BluePrints/Interface/HealthAndGold.HealthAndGold_C|GetHpVultur _ashealth_and_gold) 1))
  (switch int _returnvalue
    (:Default
      (Game|SpawnActorfromClass "/Game/BluePrints/Enemies/Mummy/Mummy.Mummy_C" (Math|Transform|MakeTransform (+ (Transformation|GetActorLocation) "0.000000,0.000000,10.000000") "0, 0, 0" "1.000000,1.000000,1.000000") "Undefined" 0 0)
      (Variables|Default|SetLast_Enemy 4))
    (:0
      (Game|SpawnActorfromClass "/Game/BluePrints/Enemies/Snake/Snake.Snake_C" (Math|Transform|MakeTransform (+ (Transformation|GetActorLocation) "0.000000,0.000000,10.000000") "0, 0, 0" "1.000000,1.000000,1.000000") "Undefined" 0 0)
      (Variables|Default|SetLast_Enemy 0))
    (:1
      (Game|SpawnActorfromClass "/Game/BluePrints/Enemies/Scorpio/Scorpio.Scorpio_C" (Math|Transform|MakeTransform (+ (Transformation|GetActorLocation) "0.000000,0.000000,10.000000") "0, 0, 0" "1.000000,1.000000,1.000000") "Undefined" 0 0)
      (Variables|Default|SetLast_Enemy 1))
    (:2
      (Game|SpawnActorfromClass "/Game/BluePrints/Enemies/Vulture/Vulture.Vulture_C" (Math|Transform|MakeTransform (+ (Transformation|GetActorLocation) "0.000000,0.000000,10.000000") "0, 0, 0" "1.000000,1.000000,1.000000") "Undefined" 0 0)
      (Variables|Default|SetLast_Enemy 2))
    (:3
      (Game|SpawnActorfromClass "/Game/BluePrints/Enemies/Hyena/Hyena.Hyena_C" (Math|Transform|MakeTransform (+ (Transformation|GetActorLocation) "0.000000,0.000000,10.000000") "0, 0, 0" "1.000000,1.000000,1.000000") "Undefined" 0 0)
      (Variables|Default|SetLast_Enemy 3))))

(event Custom|Timer%20Reset
  (if (> (Variables|Default|GetMyTime) 3.0)
    (bind _output_get (Variables|Default|SetMyTime (- (Variables|Default|GetMyTime) 0.1)))
    (bind _returnvalue (Utilities|Time|SetTimerbyEvent (delegate Custom|Spawn%20Tick) _output_get true))
    (Variables|Default|SetSpawn_Timer _returnvalue)))

(event EventBeginPlay
  (Variables|Default|SetLast_Enemy 4)
  (Variables|Default|SetMyTime 8.0)
  (bind _returnvalue (Utilities|Time|SetTimerbyEvent (delegate Custom|Spawn%20Tick) (stale Custom|Timer%20Reset _output_get) true))
  (Variables|Default|SetSpawn_Timer _returnvalue))

(fn ConstructionScript)