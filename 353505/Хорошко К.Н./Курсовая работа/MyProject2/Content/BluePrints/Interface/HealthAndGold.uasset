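; HealthAndGold is an actor that acts as a data holder for the game's gold, health and six numbered Actor variables.
; BeginPlay sets starting gold and health and initializes a Stroka string in clock format, which has no accessor functions.
; Simple getter and setter functions expose the other values, with no clamping or change notification.
; Tick, overlap and construction do nothing, and the file does not show what the Actor slots represent.
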(event EventBeginPlay
  (Variables|Default|SetGold 1000)
  (Variables|Default|SetHealth 10000)
  (Variables|Default|SetStroka "00:00"))

(event Collision|EventActorBeginOverlap
  (params (OtherActor :type Actor%20Object%20Reference)))

(event EventTick
  (params (DeltaSeconds :type Float%20%28single-precision%29)))

(fn ConstructionScript)

(fn SetGold
  (params (NewParam :type Integer))
  (Variables|Default|SetGold NewParam))

(fn GetGold
  (return (Variables|Default|GetGold)))

(fn SetHealth
  (params (NewParam :type Integer))
  (Variables|Default|SetHealth NewParam))

(fn GetHealth
  (return (Variables|Default|GetHealth)))

(fn SetActor1
  (params (NewParam :type Actor%20Object%20Reference))
  (Variables|Default|SetActor1 NewParam))

(fn GetActor1
  (return (Variables|Default|GetActor1)))

(fn SetActor2
  (params (NewParam :type Actor%20Object%20Reference))
  (Variables|Default|SetActor2 NewParam))

(fn GetActor2
  (return (Variables|Default|GetActor2)))

(fn SetActor3
  (params (NewParam :type Actor%20Object%20Reference))
  (Variables|Default|SetActor3 NewParam))

(fn GetActor3
  (return (Variables|Default|GetActor3)))

(fn SetActor4
  (params (NewParam :type Actor%20Object%20Reference))
  (Variables|Default|SetActor4 NewParam))

(fn GetActor4
  (return (Variables|Default|GetActor4)))

(fn SetActor5
  (params (NewParam :type Actor%20Object%20Reference))
  (Variables|Default|SetActor5 NewParam))

(fn GetActor5
  (return (Variables|Default|GetActor5)))

(fn SetActor6
  (params (NewParam :type Actor%20Object%20Reference))
  (Variables|Default|SetActor6 NewParam))

(fn GetActor6
  (return (Variables|Default|GetActor6)))