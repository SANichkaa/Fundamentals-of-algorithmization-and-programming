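; Bullet_DarkElf is a projectile, apparently for a Dark Elf shooter, that damages enemies on impact.
; When its Sphere component hits an actor tagged Enemy, it applies a base damage with a random roll that adds a flat bonus roughly 30% of the time, like a critical hit.
; The bullet destroys itself after any hit, whether or not the target is an enemy.
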(event OnComponentHit(Sphere)
  (params (HitComponent :type Primitive%20Component%20Object%20Reference) (OtherActor :type Actor%20Object%20Reference) (OtherComp :type Primitive%20Component%20Object%20Reference) (NormalImpulse :type Vector :default "0, 0, 0") (Hit :type Hit%20Result%20Structure%20%28by%20ref%29))
  (Variables|Default|Setdamage 25)
  (if (Actor|ActorHasTag OtherActor "Enemy")
    (bind _returnvalue (Class|Spawn|RandomMod 100))
    (Variables|Default|Setn _returnvalue)
    (if (< (Variables|Default|Getn) 30)
      (Game|Damage|ApplyDamage OtherActor (Math|Conversions|ToFloat(Integer) (+ (Variables|Default|Getdamage) 7)) 0 0)
      (else
        (Game|Damage|ApplyDamage OtherActor (Math|Conversions|ToFloat(Integer) (Variables|Default|Getdamage)) 0 0))))
  (Actor|DestroyActor))

(fn ConstructionScript)